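; BlackNote is a note actor that orbits the player's pawn horizontally.
; On BeginPlay it caches player 0's controlled pawn as its owner, moves to a set distance from it and applies a random starting angle.
; Each Tick, RotateAroundOwer accumulates the angle by rotation speed and delta time, then rebuilds the position from a Z-axis-rotated offset around the pawn's current location, so the orbit follows it.
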(event EventBeginPlay
  (Variables|Default|SetOwnerActor (Pawn|GetControlledPawn (Game|GetPlayerController 0)))
  (Transformation|SetActorLocation (Math|Vector|MakeVector (+ (Variables|Default|GetDistanceToOwner) (.x (Transformation|GetActorLocation (Variables|Default|GetOwnerActor)))) (.y (Transformation|GetActorLocation (Variables|Default|GetOwnerActor))) (.z (Transformation|GetActorLocation (Variables|Default|GetOwnerActor)))) false false)
  (CallFunction|RotateAroundOwer (* (Math|Random|RandomFloat) 3.6e+02)))

(event EventTick
  (params (DeltaSeconds :type Float%20%28single-precision%29))
  (CallFunction|RotateAroundOwer (* DeltaSeconds (Variables|Default|GetRotationSpeed))))

(fn ConstructionScript)

(fn RotateAroundOwer
  (params (Rotation :type Float%20%28double-precision%29))
  (bind _owneractor (Variables|Default|GetOwnerActor))
  (bind _returnvalue (Transformation|GetActorLocation _owneractor))
  (Variables|Default|SetCurrentRotation (+ Rotation (Variables|Default|GetCurrentRotation)))
  (Transformation|SetActorLocation (+ (Math|Vector|RotateVectorAroundAxis (- (+ (Math|Vector|MakeVector (Variables|Default|GetDistanceToOwner) 0.0 0.0) _returnvalue) _returnvalue) (Variables|Default|GetCurrentRotation) "0.000000,0.000000,1.000000") (Transformation|GetActorLocation (Variables|Default|GetOwnerActor))) false false))