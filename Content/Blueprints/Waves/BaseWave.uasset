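; BaseWave is a wave actor that grows outward in X and Y over time from a spawn radius.
; BeginPlay sets the current radius to the spawn radius, then Tick increases it by a scale speed multiplied by delta time.
; Both events call UpdateWaveMeshScale, which scales the whole actor by current over default radius, keeping Z at 1.
; The growth has no upper limit in this Blueprint.
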(event EventBeginPlay
  (Variables|Default|SetCurrentRadious (Variables|Default|GetSpawnRadious))
  (CallFunction|UpdateWaveMeshScale))

(event EventTick
  (params (DeltaSeconds :type Float%20%28single-precision%29))
  (Variables|Default|SetCurrentRadious (+ (* DeltaSeconds (Variables|Default|GetScaleSpeed)) (Variables|Default|GetCurrentRadious)))
  (CallFunction|UpdateWaveMeshScale))

(fn ConstructionScript)

(fn UpdateWaveMeshScale
  (bind _defaultradious (Variables|Default|GetDefaultRadious))
  (bind _currentradious (Variables|Default|GetCurrentRadious))
  (bind _returnvalue (/ _currentradious _defaultradious))
  (Transformation|SetActorScale3D (Math|Vector|MakeVector _returnvalue _returnvalue 1.0))
  (return))